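; Timer Blueprint that runs a stopwatch counting minutes, seconds and milliseconds.
; BeginPlay starts a looping one-millisecond timer calling Stopwatch, which increments and rolls over the counters by call count, not measured time, while IsDone is false.
; SetTime formats the Timer string and prints it, both at construction and on every count.
; An older copy of the counting logic sits unconnected in the EventGraph.
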(event EventBeginPlay
  (Utilities|Time|SetTimerbyFunctionName 0 "Stopwatch" 0.001 true))

(event Collision|EventActorBeginOverlap
  (params (OtherActor :type Actor%20Object%20Reference)))

(event EventTick
  (params (DeltaSeconds :type Float%20%28single-precision%29)))

(fn ConstructionScript
  (Utilities|SetTime))

(fn Stopwatch
  (if (not (Variables|Default|GetIsDone))
    (Math|Integer|IncrementInt (Variables|Default|GetMiliSecond)
      (:%20%20
        (if (== (Variables|Default|GetMiliSecond) 1000)
          (Variables|Default|SetMiliSecond 0)
          (Math|Integer|IncrementInt (Variables|Default|GetSecond)
            (:%20%20
              (if (== (Variables|Default|GetSecond) 60)
                (Variables|Default|SetSecond 0)
                (Math|Integer|IncrementInt (Variables|Default|GetMinute)
                  (:%20%20
                    (Utilities|SetTime)))
                (else
                  (Utilities|SetTime)))))
          (else
            (Utilities|SetTime)))))))