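; BP_Cube is a short-lived cube actor that gets a random color when play begins.
; BeginPlay rolls an integer from 0 to 3 to set a red, green or blue material, leaving the existing material on a 3.
; Tick accumulates time and destroys the actor after ten seconds, while any overlap on the cube component destroys it immediately.
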(event OnComponentBeginOverlap(GC_RedCube)
  (params (OverlappedComponent :type Primitive%20Component%20Object%20Reference) (OtherActor :type Actor%20Object%20Reference) (OtherComp :type Primitive%20Component%20Object%20Reference) (OtherBodyIndex :type Integer) (bFromSweep :type Boolean) (SweepResult :type Hit%20Result%20Structure%20%28by%20ref%29))
  (Actor|DestroyActor))

(event EventBeginPlay
  (bind _gc_redcube (Variables|Default|GetGC_RedCube))
  (Variables|Default|SetCurrentTime 0.0)
  (Variables|Default|SetDestroyTime 1e+01)
  (bind _output_get (Variables|Default|SetRandom (Math|Random|RandomIntegerinRange 0 3)))
  ;[0.15 0.15 0.15 0.5] 0 == Red
  (if (== _output_get 0)
    (Rendering|Material|SetMaterial _gc_redcube 0 "/Game/Ksk/Materials/Red.Red")
    (else
      ;[0.15 0.15 0.15 0.5] 1 == Green
      (if (== _output_get 1)
        (Rendering|Material|SetMaterial _gc_redcube 0 "/Game/Ksk/Materials/Green.Green")
        (else
          ;[0.15 0.15 0.15 0.5] 2 == Blue
          (if (== _output_get 2)
            (Rendering|Material|SetMaterial _gc_redcube 0 "/Game/Ksk/Materials/Blue.Blue")))))))

(event Collision|EventActorBeginOverlap
  (params (OtherActor :type Actor%20Object%20Reference)))

(event EventTick
  (params (DeltaSeconds :type Float%20%28single-precision%29))
  (bind _output_get (Variables|Default|SetCurrentTime (+ DeltaSeconds (Variables|Default|GetCurrentTime))))
  (if (> _output_get (Variables|Default|GetDestroyTime))
    (Actor|DestroyActor)))

(fn ConstructionScript)