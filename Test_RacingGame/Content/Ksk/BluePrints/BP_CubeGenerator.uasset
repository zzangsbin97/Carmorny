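; BP_CubeGenerator is a spawner actor that creates BP_Cube actors at its own location on a repeating timer.
; Tick accumulates delta time in CurrentTime and, once it exceeds CreateTime, resets it to zero and spawns a cube.
; BeginPlay seeds CurrentTime with a nonzero value, so the first spawn comes early or immediately, depending on CreateTime.
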(event EventBeginPlay
  (Variables|Default|SetCurrentTime 1e+01))

(event Collision|EventActorBeginOverlap
  (params (OtherActor :type Actor%20Object%20Reference)))

(event EventTick
  (params (DeltaSeconds :type Float%20%28single-precision%29))
  (bind _output_get (Variables|Default|SetCurrentTime (+ DeltaSeconds (Variables|Default|GetCurrentTime))))
  ;[0.15 0.15 0.15 0.5] Reset Timer
  (if (> _output_get (Variables|Default|GetCreateTime))
    (Variables|Default|SetCurrentTime 0.0)
    (Game|SpawnActorfromClass "/Game/Ksk/BluePrints/BP_Cube.BP_Cube_C" (Math|Conversions|ToTransform(Vector) (Transformation|GetActorLocation)) "Undefined" "MultiplyWithRoot" 0 0)))

(fn ConstructionScript)