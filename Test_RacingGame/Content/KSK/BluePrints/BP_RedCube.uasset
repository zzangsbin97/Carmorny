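; BP_RedCube is a red cube pickup for a vehicle game that self-destructs about ten seconds after spawning.
; Tick accumulates elapsed time and destroys the actor once it exceeds DestroyTime.
; When GC_RedCube overlaps a SportsCar_Pawn, it prints a debug string, calls RedCubeCountIncrease on the VehiclePlayerController, then destroys itself.
; The controller comes from GetPlayerControllerFromInputDevice rather than the overlapping pawn.
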(event OnComponentBeginOverlap(GC_RedCube)
  (params (OverlappedComponent :type Primitive%20Component%20Object%20Reference) (OtherActor :type Actor%20Object%20Reference) (OtherComp :type Primitive%20Component%20Object%20Reference) (OtherBodyIndex :type Integer) (bFromSweep :type Boolean) (SweepResult :type Hit%20Result%20Structure%20%28by%20ref%29))
  (Development|PrintString "Red Overlap")
  (Utilities|Casting|CastToSportsCar_Pawn OtherActor)
  (bind _returnvalue (Class|InputDeviceLibrary|GetPlayerControllerfromInputDevice))
  (bind _asvehicle_player_controller (Utilities|Casting|CastToVehiclePlayerController _returnvalue))
  (Default|RedCubeCountIncrease _asvehicle_player_controller)
  (Actor|DestroyActor))

(event EventBeginPlay
  (Variables|Default|SetCurrentTime 0.0)
  (Variables|Default|SetDestroyTime 1e+01))

(event Collision|EventActorBeginOverlap
  (params (OtherActor :type Actor%20Object%20Reference)))

(event EventTick
  (params (DeltaSeconds :type Float%20%28single-precision%29))
  (bind _output_get (Variables|Default|SetCurrentTime (+ DeltaSeconds (Variables|Default|GetCurrentTime))))
  (if (> _output_get (Variables|Default|GetDestroyTime))
    (Actor|DestroyActor)))

(fn ConstructionScript)